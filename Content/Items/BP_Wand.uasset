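; BP_Wand is a wand item Blueprint that supplies its own default item data.
; GetDefaultItem constructs an ItemData object and initialises it with a one-by-three footprint, the wand icon and a reference to BP_Wand.
; The event graph holds only disabled placeholder events, and the construction script just calls its parent.
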(fn `GetDefaultItem`
  (returns (ReturnValue :type "ItemData Object Reference"))
  (bind _returnvalue (`|GenericCreateObject` "/Script/Unreal_RPG.ItemData" self))
  (`ItemData.Initialise` _returnvalue (1.0 3.0) "/Game/Items/wandIcon.wandIcon" "BP_Wand_C")
  (return _returnvalue))

(fn `UserConstructionScript`
  (`parent.UserConstructionScript`))